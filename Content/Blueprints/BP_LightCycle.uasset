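; Tron-style light cycle that constantly accelerates under physics, steers by externally set yaw input and self-rights roll and pitch.
; While moving fast enough, it periodically extends a spawned BP_LightWall as trail collision, alongside a colored ribbon.
; Moving too slowly or losing speed sharply on impact drains health, which regenerates after a delay.
; Death notifies BP_GameMode, fires a color-matched Niagara explosion and destroys the meshes.
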(event `self.ReceiveBeginPlay`
  ;[1 1 1] Add LightWall blueprint
  (bind _returnvalue (`|SpawnActorFromClass` "/Game/Blueprints/BP_LightWall.BP_LightWall_C" (`KismetMathLibrary.MakeTransform` (0.0 0.0 0.0)) "AlwaysSpawn" "OverrideRootScale" null null))
  (set `self.BP_LightWall` _returnvalue)
  (set `self.LW_LastTransformLocation` (+ (`SceneComponent.K2_GetComponentLocation` (`self.SM_LightCycle`)) (`KismetMathLibrary.MakeVector` (`self.LW_SpawnOffset`)))))

(event `self.ReceiveTick`
  (params (DeltaSeconds :type "Float (single-precision)"))
  (bind _sm_lightcycle (`self.SM_LightCycle`))
  (bind _tiltupspeed (`self.TiltUpSpeed`))
  (bind _sm_lightcycle_2 (`self.SM_LightCycle`))
  (bind (_relativerotation_roll _relativerotation_pitch _relativerotation_yaw) (`KismetMathLibrary.BreakRotator` (`SceneComponent.RelativeRotation` _sm_lightcycle)))
  (`SceneComponent.K2_SetRelativeRotation` _sm_lightcycle (`KismetMathLibrary.MakeRotator` (`KismetMathLibrary.Lerp` _relativerotation_roll 0.0 _tiltupspeed) (`KismetMathLibrary.Lerp` _relativerotation_pitch 0.0 _tiltupspeed) _relativerotation_yaw) false false)
  (if (`self.IsEnabled`)
    ;[1 1 1] Force throttle and handle input
    (`self.Throttle` 1.0)
    (`self.Steer` (`self.LastSteerValue`))
    (bind _returnvalue (`PrimitiveComponent.GetPhysicsLinearVelocity` (`self.SM_LightCycle`) "None"))
    (set `self.LastVelocity` _returnvalue)
    (set `self.LW_LastSpawnTime` (+ (`self.LW_LastSpawnTime`) DeltaSeconds))
    (if (> (`self.LW_LastSpawnTime`) (`self.LW_SpawnRate`))
      (set `self.LW_LastSpawnTime` 0.0)
      (`self.CompareCurrentVelocityToFloat` (`self.LW_MinSpawnVelocity`)
        (:`IsGreater`
          (`LightWall.ExtendLightWall` (`self.BP_LightWall`) (+ (`SceneComponent.K2_GetComponentLocation` _sm_lightcycle_2) (`KismetMathLibrary.GreaterGreater_VectorRotator` (`KismetMathLibrary.MakeVector` (`self.LW_SpawnOffset`)) (`SceneComponent.K2_GetComponentRotation` _sm_lightcycle_2)))))
        (:`IsSmaller`
          _)
        (:`IsEqual`
          _)))
    ;[1 1 1] Check if damage should be applied
    (`self.CompareCurrentVelocityToFloat` (`self.Health_MinVelocity`)
      (:`IsGreater`
        _)
      (:`IsSmaller`
        (`self.Do Damage` (* (`self.Health_MinVelocityDamage`) DeltaSeconds)))
      (:`IsEqual`
        _))
    (bind _output_get (set `self.Health_RegenerationTime` (+ (`self.Health_RegenerationTime`) DeltaSeconds)))
    (if (>= _output_get (`self.Health_RegenerationDelay`))
      (set `self.Health` (`KismetMathLibrary.FMin` (+ (`self.Health`) (* (`self.Health_RegenerationSpeed`) DeltaSeconds)) 100.0)))))

(event `self.SM_LightCycle.OnComponentHit`
  (params (HitComponent :type "PrimitiveComponent Object Reference") (OtherActor :type "Actor Object Reference") (OtherComp :type "PrimitiveComponent Object Reference") (NormalImpulse :type "Vector Structure") (Hit :type "HitResult Structure (by ref)"))
  ;[1 1 1] Check if an in damage resulting object was hit
  (if (`self.IsEnabled`)
    (if (not (`self.IsDead`))
      ;[1 1 1] Calculate damage due to collision
      (if (`KismetArrayLibrary.Array_Contains` (`|MakeArray` "ECC_GameTraceChannel1" "ECC_WorldStatic" :!type "ECollisionChannel Enum") (`PrimitiveComponent.GetCollisionObjectType` OtherComp))
        (bind _returnvalue (`PrimitiveComponent.GetPhysicsLinearVelocity` (`self.SM_LightCycle`) "None"))
        (bind _returnvalue_2 (`KismetMathLibrary.FMax` (- (`KismetMathLibrary.VSize` (`self.LastVelocity`)) (`KismetMathLibrary.VSize` _returnvalue))))
        (if (> _returnvalue_2 700.0)
          (bind _returnvalue_3 (`KismetMathLibrary.FFloor` (* _returnvalue_2 (`self.Health_DamageFactor`))))
          (if (> _returnvalue_3 0)
            (`self.Do Damage` (`KismetMathLibrary.Conv_IntToDouble` _returnvalue_3))))))))

(event `OnDeath`
  (bind _ns_explosion (`self.NS_Explosion`))
  (if (`self.IsEnabled`)
    (if (not (`self.IsDead`))
      (set `self.IsDead` true)
      (bind _asbp_game_mode (cast `/Game/Blueprints/BP_GameMode` (`GameplayStatics.GetGameMode`)))
      (`/Game/Blueprints/BP_GameMode.LightCycleDestroyed` _asbp_game_mode self)
      ;[1 1 1] Show explosion and hide light cycle
      (`FXSystemComponent.SetVectorParameter` _ns_explosion "ExplosionColor" (`KismetMathLibrary.Conv_LinearColorToVector` (`self.Color`)))
      (`ActorComponent.Activate` _ns_explosion false)
      (`self.SetActorTickEnabled` false)
      (`KismetSystemLibrary.Delay` 0.2)
      (`ActorComponent.K2_DestroyComponent` (`self.SkeletalMesh`))
      (`ActorComponent.K2_DestroyComponent` (`self.SM_LightCycle`)))))

(fn `Do Damage`
  (params (DamageAmount :type "Float (double-precision)"))
  (set `self.Health_RegenerationTime` 0.0)
  (bind _output_get (set `self.Health` (`KismetMathLibrary.FMax` (- (`self.Health`) DamageAmount))))
  (if (<= _output_get 0.0)
    (`self.OnDeath`)))

(fn `SetLightColor`
  (params (LinearColor :type "LinearColor Structure"))
  (set `self.Color` LinearColor)
  ;[1 1 1] Set material color
  (`MaterialInstanceDynamic.SetVectorParameterValue` (`self.Material`) "Input" LinearColor)
  ;[1 1 1] Set light trail color
  (`FXSystemComponent.SetColorParameter` (`self.PS_Ribbon`) "Color" LinearColor))

(fn `SetSteer`
  (params (SteerAxisValue :type "Float (double-precision)"))
  (set `self.LastSteerValue` SteerAxisValue))

(fn `Steer`
  (params (AxisValue :type "Float (double-precision)"))
  (bind _sm_lightcycle (`self.SM_LightCycle`))
  (bind (_relativerotation_roll _relativerotation_pitch _relativerotation_yaw) (`KismetMathLibrary.BreakRotator` (`SceneComponent.RelativeRotation` _sm_lightcycle)))
  (`SceneComponent.K2_AddRelativeRotation` _sm_lightcycle (`KismetMathLibrary.MakeRotator` 0.0 0.0 (* AxisValue (`self.SteerStrength`))) false false)
  (`PrimitiveComponent.AddForce` _sm_lightcycle (`KismetMathLibrary.GreaterGreater_VectorRotator` (* (0.0 1.0 0.0) (* 0.0 (`self.SteerForce`))) (`KismetMathLibrary.MakeRotator` 0.0 0.0 _relativerotation_yaw)) "None" true))

(fn `Throttle`
  (params (AxisValue :type "Float (double-precision)"))
  (bind _sm_lightcycle (`self.SM_LightCycle`))
  (bind (_returnvalue_roll _returnvalue_pitch _returnvalue_yaw) (`KismetMathLibrary.BreakRotator` (`SceneComponent.K2_GetComponentRotation` _sm_lightcycle)))
  (`PrimitiveComponent.AddForce` _sm_lightcycle (`KismetMathLibrary.GreaterGreater_VectorRotator` (* (1.0 0.0 0.0) (* AxisValue (`self.MovementSpeed`))) (`KismetMathLibrary.MakeRotator` 0.0 0.0 _returnvalue_yaw)) "None" true))

(fn `UserConstructionScript`
  (bind _skeletalmesh (`self.SkeletalMesh`))
  ;[1 1 1] Create material instance
  (bind _returnvalue (`KismetMaterialLibrary.CreateDynamicMaterialInstance` "/Game/Materials/M_LightCycleStripes.M_LightCycleStripes"))
  (bind _output_get (set `self.Material` _returnvalue))
  (`PrimitiveComponent.SetMaterial` _skeletalmesh 2 _output_get)
  (`PrimitiveComponent.SetMaterial` _skeletalmesh 4 _output_get)
  (`PrimitiveComponent.SetMaterial` _skeletalmesh 6 _output_get)
  (`PrimitiveComponent.SetMaterial` _skeletalmesh 7 _output_get))