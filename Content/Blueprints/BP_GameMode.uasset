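; Game mode for a light cycle match that runs a timed start and decides when players lose or win.
; BeginPlay gathers all cycles and player controllers, gives cycles shuffled colors and disables them; Tick counts up to StartDelay, then enables them once.
; LightCycleDestroyed drops the cycle and any owning controller, showing that player a death screen.
; When one cycle and one controller remain, that player gets the win screen and its cycle is disabled.
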(event `self.ReceiveBeginPlay`
  (bind _outactors (`GameplayStatics.GetAllActorsOfClass` "/Game/Blueprints/BP_LightCycle.BP_LightCycle_C"))
  (set `self.BP_LightCycleList` _outactors)
  (bind _outactors_2 (`GameplayStatics.GetAllActorsOfClass` "/Game/Blueprints/BP_PlayerController.BP_PlayerController_C"))
  (set `self.BP_PlayerControllers` _outactors_2)
  (`KismetArrayLibrary.Array_Shuffle` (`self.Colors`))
  (for (_array_element _array_index) (`self.BP_LightCycleList`)
    (`/Game/Blueprints/BP_LightCycle.SetLightColor` _array_element (`|GetArrayItem` (`self.Colors`) _array_index))
    (set `/Game/Blueprints/BP_LightCycle.IsEnabled` false _array_element)))

(event `self.ReceiveTick`
  (params (DeltaSeconds :type "Float (single-precision)"))
  (bind _output_get (set `self.Time` (+ (`self.Time`) DeltaSeconds)))
  (if (>= _output_get (`self.StartDelay`))
    (`self.OnStartCompleted`)))

(event `OnStartCompleted`
  (if (not (`self.IsStartCompleted`))
    (set `self.IsStartCompleted` true)
    (for _array_element (`self.BP_LightCycleList`)
      (set `/Game/Blueprints/BP_LightCycle.IsEnabled` true _array_element))))

(fn `FindPlayerController`
  (params (BP_LightCycle :type "/Game/Blueprints/BP_LightCycle Object Reference"))
  (returns (BP_PlayerController :type "/Game/Blueprints/BP_PlayerController Object Reference"))
  (for _array_element (`self.BP_PlayerControllers`)
    (if (== (`/Game/Blueprints/BP_PlayerController.LightCycle` _array_element) BP_LightCycle)
      (return _array_element)))
  (return null))

(fn `LightCycleDestroyed`
  (params (BP_LightCycle :type "/Game/Blueprints/BP_LightCycle Object Reference"))
  (locals (destroyedLightCycle :type "/Game/Blueprints/BP_LightCycle Object Reference"))
  (bind _bp_playercontrollers (`self.BP_PlayerControllers`))
  (bind _output (`|GetArrayItem` _bp_playercontrollers))
  (bind _lightcycle (`/Game/Blueprints/BP_PlayerController.LightCycle` _output))
  (bind _bp_playercontroller (`self.FindPlayerController` BP_LightCycle))
  (`KismetArrayLibrary.Array_RemoveItem` (`self.BP_LightCycleList`) BP_LightCycle)
  ;[1 1 1] If a player died, show death screen
  (if (`KismetSystemLibrary.IsValid` _bp_playercontroller)
    (`KismetArrayLibrary.Array_RemoveItem` (`self.BP_PlayerControllers`) _bp_playercontroller)
    (`/Game/Blueprints/BP_PlayerController.ShowScreen` _bp_playercontroller "NewEnumerator0"))
  ;[1 1 1] If only one player remains, show win screen
  (if (and (== (`KismetArrayLibrary.Array_Length` (`self.BP_LightCycleList`)) 1) (== (`KismetArrayLibrary.Array_Length` _bp_playercontrollers) 1))
    (if (`/Game/Blueprints/BP_LightCycle.IsEnabled` _lightcycle)
      (`/Game/Blueprints/BP_PlayerController.ShowScreen` _output "NewEnumerator1")
      (set `/Game/Blueprints/BP_LightCycle.IsEnabled` false _lightcycle))))

(fn `UserConstructionScript`)