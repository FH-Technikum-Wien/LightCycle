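; Player controller for the light cycle pawn, handling steering input, camera control and the player's UI.
; Camera axis inputs rotate the spring arm, which lerps back to its saved starting rotation once input idles past a cooldown timed on Tick.
; Tick also feeds the cycle's health to the HUD.
; ShowScreen replaces all widgets with a death or win screen and switches to UI-only input with a cursor.
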(event `self.ReceiveBeginPlay`
  ;[1 1 1] Get LightCycle reference
  (bind _asbp_light_cycle (cast `/Game/Blueprints/BP_LightCycle` (`self.K2_GetPawn`)))
  (set `self.LightCycle` _asbp_light_cycle)
  ;[1 1 1] Save start position of camera
  (set `self.CameraDefaultPosition` (`SceneComponent.RelativeRotation` (`/Game/Blueprints/BP_LightCycle.SpringArm` (`self.LightCycle`))))
  ;[1 1 1] Show Player HUD
  (bind _returnvalue (`|CreateWidget` "/Game/UI/W_PlayerHUD.W_PlayerHUD_C" self))
  (bind _output_get (set `self.PlayerHUD` _returnvalue))
  (`UserWidget.AddToViewport` _output_get 0)
  (`WidgetBlueprintLibrary.SetInputMode_GameOnly` (`GameplayStatics.GetPlayerController` 0)))

(event `self.ReceiveTick`
  (params (DeltaSeconds :type "Float (single-precision)"))
  ;[1 1 1] Update last camera reset time
  (set `self.CameraResetTime` (+ DeltaSeconds (`self.CameraResetTime`)))
  ;[1 1 1] Update HUD health
  (set `/Game/UI/W_PlayerHUD.HealthPercentage` (/ (`/Game/Blueprints/BP_LightCycle.Health` (`self.LightCycle`)) 100.0) (`self.PlayerHUD`)))

(event `InputAxis|InputCameraUpDown`
  (params (AxisValue :type "Float (single-precision)"))
  (bind _camerasensitivity (`self.CameraSensitivity`))
  (bind _springarm (`/Game/Blueprints/BP_LightCycle.SpringArm` (`self.LightCycle`)))
  ;[1 1 1] Camera Controls
  (`SceneComponent.K2_AddRelativeRotation` (`/Game/Blueprints/BP_LightCycle.SpringArm` (`self.LightCycle`)) (`KismetMathLibrary.MakeRotator` 0.0 (* AxisValue _camerasensitivity) (* _camerasensitivity (stale `InputAxis|InputCameraLeftRight` AxisValue))) false false :!label _label)
  (if (or (< (`KismetMathLibrary.Abs` AxisValue) 0.1) (< (`KismetMathLibrary.Abs` (stale `InputAxis|InputCameraLeftRight` AxisValue)) 0.1))
    (if (> (`self.CameraResetTime`) (`self.CameraResetCooldown`))
      (`SceneComponent.K2_SetRelativeRotation` _springarm (`KismetMathLibrary.RLerp` (`SceneComponent.RelativeRotation` _springarm) (`self.CameraDefaultPosition`) (`self.CameraReturnSpeed`)) false false))
    (else
      (set `self.CameraResetTime` 0.0))))

(event `InputAxis|InputCameraLeftRight`
  (params (AxisValue :type "Float (single-precision)"))
  ;[1 1 1] Camera Controls
  (goto _label))

(event `InputAxis|InputMovementLeftRight`
  (params (AxisValue :type "Float (single-precision)"))
  ;[1 1 1] Movement
  (set `self.IsReceivingSteer` (> (`KismetMathLibrary.Abs` AxisValue) 0.0))
  (`/Game/Blueprints/BP_LightCycle.SetSteer` (`self.LightCycle`) AxisValue))

(fn `ShowScreen`
  (params (PlayerScreen :type "/Game/Blueprints/Enum_PlayerScreens Enum" :default "NewEnumerator0"))
  (bind _returnvalue (`GameplayStatics.GetPlayerController` 0))
  (`WidgetLayoutLibrary.RemoveAllWidgets`)
  (switch `/Game/Blueprints/Enum_PlayerScreens` PlayerScreen
    (:`NewEnumerator0`
      (bind _returnvalue_2 (`|CreateWidget` "/Game/UI/W_DeathScreen.W_DeathScreen_C" self))
      (`UserWidget.AddToViewport` _returnvalue_2 0))
    (:`NewEnumerator1`
      (bind _returnvalue_3 (`|CreateWidget` "/Game/UI/W_WinScreen.W_WinScreen_C" self))
      (`UserWidget.AddToViewport` _returnvalue_3 0)))
  (`WidgetBlueprintLibrary.SetInputMode_UIOnlyEx` _returnvalue null)
  (set `PlayerController.bShowMouseCursor` true _returnvalue))

(fn `UserConstructionScript`)