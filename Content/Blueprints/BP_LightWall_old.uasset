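; BP_LightWall_old is an actor that builds a hidden, collidable wall along a trail of points.
; CreateLightWall appends a vertex pair at the given location and LightWallHeight above it, then offsets a TriangleIndices template to extend the triangle list once enough vertices exist.
; Each call clears and recreates the entire PMTrail procedural mesh section with collision, then hides it.
; Its events and construction script are empty, so CreateLightWall relies on external callers.
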(fn `CreateLightWall`
  (params (ToLocation :type "Vector Structure"))
  (locals (TempVertices :type "Array of Vector Structure") (TempTriangles :type "Array of Integer"))
  (bind _pmtrail (`self.PMTrail`))
  (if (> (`KismetArrayLibrary.Array_Length` (`self.Vertices`)) 2)
    (set `self.wallSegmentCount` (+ (`self.wallSegmentCount`) 2))
    (for _array_element (`self.TriangleIndices`)
      (`KismetArrayLibrary.Array_Add` (`self.Triangles`) (+ _array_element (`self.wallSegmentCount`)))))
  (`KismetArrayLibrary.Array_Append` (`self.Vertices`) (`|MakeArray` ToLocation (+ ToLocation (`KismetMathLibrary.MakeVector` 0.0 0.0 (`self.LightWallHeight`)))))
  (`ProceduralMeshComponent.ClearMeshSection` _pmtrail 0)
  (`ProceduralMeshComponent.CreateMeshSection_LinearColor` :`self` _pmtrail :`Vertices` (`self.Vertices`) :`Triangles` (`self.Triangles`) :`bCreateCollision` true)
  (`ProceduralMeshComponent.SetMeshSectionVisible` (`self.PMTrail`) 0 false))

(fn `UserConstructionScript`)